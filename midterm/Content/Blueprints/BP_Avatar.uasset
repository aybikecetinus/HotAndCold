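; BP_Avatar is a player-controlled character with walking, running, stamina and a heavy attack, driven by Enhanced Input.
; Move input follows control yaw, while look input only turns yaw.
; Tick drains stamina during running and regenerates it otherwise; full depletion forces walk speed until stamina refills completely.
; ChangeState extends the parent, then uses the anim state to lock movement during attacks and death, also disabling orient-to-movement for attacks.
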(event Input|EnhancedActionEvents|EnhancedInputActionIA_Look
  (params (ActionValue :type Vector%202D%20Structure) (ElapsedSeconds :type Float%20%28double-precision%29) (TriggeredSeconds :type Float%20%28double-precision%29) (InputAction :type Input%20Action%20Object%20Reference :default "/Game/ThirdPerson/Input/Actions/IA_Look.IA_Look"))
  (:Triggered
    (Pawn|Input|AddControllerYawInput (.x ActionValue))
    (Pawn|Input|AddControllerPitchInput 0.0)))

(event Input|EnhancedActionEvents|EnhancedInputActionIA_HeavyAttack
  (params (ActionValue :type Boolean) (ElapsedSeconds :type Float%20%28double-precision%29) (TriggeredSeconds :type Float%20%28double-precision%29) (InputAction :type Input%20Action%20Object%20Reference :default "/Game/ThirdPerson/Input/Actions/IA_HeavyAttack.IA_HeavyAttack"))
  (:Triggered
    (CallFunction|ChangeState "NewEnumerator10")
    (Variables|Default|SetHeavyAttackTriggered true)))

(event Input|EnhancedActionEvents|EnhancedInputActionIA_Run
  (params (ActionValue :type Boolean) (ElapsedSeconds :type Float%20%28double-precision%29) (TriggeredSeconds :type Float%20%28double-precision%29) (InputAction :type Input%20Action%20Object%20Reference :default "/Game/ThirdPerson/Input/Actions/IA_Run.IA_Run"))
  (:Triggered
    (Variables|Default|SetRunning true)
    (CallFunction|UpdateMovementParameter :!label _label))
  (:Completed
    (Variables|Default|SetRunning false)
    (goto _label)))

(event Input|EnhancedActionEvents|EnhancedInputActionIA_Move
  (params (ActionValue :type Vector%202D%20Structure) (ElapsedSeconds :type Float%20%28double-precision%29) (TriggeredSeconds :type Float%20%28double-precision%29) (InputAction :type Input%20Action%20Object%20Reference :default "/Game/ThirdPerson/Input/Actions/IA_Move.IA_Move"))
  (bind _returnvalue (Pawn|GetControlRotation :!class /Script/Engine.Pawn))
  (bind _movementscale (Variables|Default|GetMovementScale))
  (bind _returnvalue_2 (Math|Rotator|MakeRotator 0.0 0.0 (.yaw _returnvalue)))
  (:Triggered
    (Pawn|Input|AddMovementInput (Math|Vector|GetRightVector _returnvalue_2) (* (.x ActionValue) _movementscale) false)
    (Pawn|Input|AddMovementInput (Math|Vector|GetForwardVector _returnvalue_2) (* (.y ActionValue) _movementscale) false)))

(event EventBeginPlay
  (|CallParentFunction)
  (Variables|Default|SetMaxStamina (Variables|Default|GetMaxStamina))
  (bind _asplayer_controller (Utilities|Casting|CastToPlayerController (Pawn|GetController)))
  (Utilities|IsValid (PlayerController|LocalPlayerSubsystems|GetEnhancedInputLocalPlayerSubsystem _asplayer_controller)
    (:Is%20Valid
      (Input|AddMappingContext (PlayerController|LocalPlayerSubsystems|GetEnhancedInputLocalPlayerSubsystem _asplayer_controller) "/Game/ThirdPerson/Input/IMC_Default.IMC_Default" 0 "(bIgnoreAllPressedKeysUntilRelease=True,bForceImmediately=False)"))))

(event Collision|EventActorBeginOverlap
  (params (OtherActor :type Actor%20Object%20Reference))
  (|CallParentFunction OtherActor) ; This node is disabled and will not be called.\nDrag off pins to build functionality.
)

(event EventTick
  (params (DeltaSeconds :type Float%20%28single-precision%29))
  (|CallParentFunction DeltaSeconds)
  (CallFunction|UpdateStamina DeltaSeconds))

(fn ConstructionScript
  (|CallParentFunction))

(fn UpdateStamina
  (params (TimeElapsed :type Float%20%28double-precision%29))
  (if (Variables|Default|GetStaminaDrained)
    (bind _output_get (Variables|Default|SetStamina (Math|Float|Min(Float) (Variables|Default|GetMaxStamina) (+ (* (Variables|Default|GetStaminaGainRate) TimeElapsed) (Variables|Default|GetStamina))) :!label _label))
    (if (== _output_get (Variables|Default|GetMaxStamina))
      (Variables|Default|SetStaminaDrained false)
      (CallFunction|UpdateMovementParameter :!label _label_2))
    (elif (and (Utilities|Enum|Equal(Enum) (Variables|/Script/Engine.CharacterMovementComponent|GetMovementMode (Variables|Character|GetCharacterMovement)) "MOVE_Walking") (> (Math|Vector|VectorLength (Transformation|GetVelocity)) 5.0))
      (if (Variables|Default|GetRunning)
        (bind _output_get_2 (Variables|Default|SetStamina (Math|Float|Max(Float) (- (Variables|Default|GetStamina) (* TimeElapsed (Variables|Default|GetStaminaDrainRate))) 0.0)))
        (if (== _output_get_2 0.0)
          (Variables|Default|SetStaminaDrained true)
          (goto _label_2))
        (else
          (goto _label)))
      (else
        (goto _label)))))

(fn UpdateMovementParameter
  (Variables|/Script/Engine.CharacterMovementComponent|SetMaxWalkSpeed (Variables|Character|GetCharacterMovement) (Math|Float|SelectFloat (Variables|Default|GetRunSpeed) (Variables|Default|GetWalkSpeed) (and (Variables|Default|GetRunning) (not (Variables|Default|GetStaminaDrained))))))

(fn ChangeState
  (params (New%20State :type E_CharAnimStates%20Enum :default "NewEnumerator0"))
  (bind _charactermovement (Variables|Character|GetCharacterMovement))
  (bind _anim (Variables|Default|GetAnim)
    (:then
      (|CallParentFunction New%20State)
      (switch Utilities|FlowControl|Switch|SwitchonE_CharAnimStates (Variables|/Game/Blueprints/AnimBP_Character.AnimBP_Character_C|GetAnimState _anim)
        (:NewEnumerator1
          (Variables|/Script/Engine.CharacterMovementComponent|SetbOrientRotationToMovement _charactermovement true)
          (Variables|Default|SetMovementScale 1.0))
        (:NewEnumerator4
          (Variables|/Script/Engine.CharacterMovementComponent|SetbOrientRotationToMovement _charactermovement false)
          (Variables|Default|SetMovementScale 0.0 :!label _label))
        (:NewEnumerator8
          (Variables|Default|SetMovementScale 0.0))
        (:NewEnumerator10
          (Variables|/Script/Engine.CharacterMovementComponent|SetbOrientRotationToMovement _charactermovement false)
          (goto _label))))
    (:else)))