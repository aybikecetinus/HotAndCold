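; Base character Blueprint for melee combat, handling health, damage, death and animation states through AnimBP_Character.
; ChangeState starts attack animations and a start-up timer that damages enemies overlapping AttackArea within a forward cone; Damage or Death cancels that timer.
; Incoming damage triggers a hit reaction and doubles while the player avatar's heavy-attack flag is set.
; Death disables input and animates only for player-controlled characters; healing exists but is not called here.
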(event Input|EnhancedActionEvents|EnhancedInputActionIA_Attack
  (params (ActionValue :type Boolean) (ElapsedSeconds :type Float%20%28double-precision%29) (TriggeredSeconds :type Float%20%28double-precision%29) (InputAction :type Input%20Action%20Object%20Reference :default "/Game/ThirdPerson/Input/Actions/IA_Attack.IA_Attack"))
  (:Triggered
    (CallFunction|ChangeState "NewEnumerator4")))

(event EventBeginPlay
  (Variables|/Script/Engine.CharacterMovementComponent|SetMaxWalkSpeed (Variables|Character|GetCharacterMovement) (Variables|Default|GetWalkSpeed))
  (Variables|Default|SetHealth (Variables|Default|GetMaxHealth))
  (bind _asanim_bp_character (Utilities|Casting|CastToAnimBP_Character (Components|SkeletalMesh|GetAnimInstance (Variables|Character|GetMesh))))
  (Variables|Default|SetAnim _asanim_bp_character)
  (bind _asbp_avatar (Utilities|Casting|CastToBP_Avatar (Game|Player|GetPlayerPawn 0)))
  (Variables|BP_BaseCharacter_C|SetAs%20BP%20Avatar _asbp_avatar 0))

(event Collision|EventActorBeginOverlap
  (params (OtherActor :type Actor%20Object%20Reference)))

(event EventTick
  (params (DeltaSeconds :type Float%20%28single-precision%29)))

(event Game|Damage|EventAnyDamage
  (params (Damage :type Float%20%28single-precision%29) (DamageType :type Damage%20Type%20Object%20Reference) (InstigatedBy :type Controller%20Object%20Reference) (DamageCauser :type Actor%20Object%20Reference))
  (if (not (Variables|Default|GetDead))
    (bind _modifieddamage (CallFunction|ModifyDamage Damage))
    (bind _output_get (Variables|Default|SetHealth (- (Variables|Default|GetHealth) _modifieddamage)))
    (if (< _output_get 0.0)
      (Variables|Default|SetDead true)
      (if (Pawn|IsPlayerControlled)
        (Input|DisableInput (Game|GetPlayerController 0))
        (CallFunction|ChangeState "NewEnumerator8")))))

(fn ConstructionScript
  (Components|Sphere|SetSphereRadius (Variables|Default|GetAttackArea) (Variables|Default|GetAttackRadius) true))

(fn UpdateHealth
  (params (TimeElapsed :type Float%20%28double-precision%29))
  (if (not (Variables|Default|GetDead))
    (Variables|Default|SetHealth (Math|Float|Min(Float) (+ (* TimeElapsed (Variables|Default|GetHealingRate)) (Variables|Default|GetHealth)) (Variables|Default|GetMaxHealth)))))

(fn ChangeState
  (params (New%20State :type E_CharAnimStates%20Enum :default "NewEnumerator0"))
  (bind _anim (Variables|Default|GetAnim))
  (bind _anim_2 (Variables|Default|GetAnim))
  (Utilities|IsValid _anim_2
    (:Is%20Valid
      (if (not (Utilities|Enum|Equal(Enum) (Variables|/Game/Blueprints/AnimBP_Character.AnimBP_Character_C|GetAnimState _anim_2) New%20State))
        (switch Utilities|FlowControl|Switch|SwitchonE_CharAnimStates New%20State
          (:NewEnumerator4
            (if (Utilities|Enum|Equal(Enum) (Variables|/Game/Blueprints/AnimBP_Character.AnimBP_Character_C|GetAnimState (Variables|Default|GetAnim)) "NewEnumerator1")
              (Default|ChangeAnimStates _anim "NewEnumerator4" (Variables|Default|GetAttackSpeed))
              (Utilities|Time|SetTimerbyFunctionName 0 "Attackk" (Variables|Default|GetAttack1StartUpDelay))))
          (:NewEnumerator7
            (Default|ChangeAnimStates _anim "NewEnumerator7" 2.0)
            (Utilities|Time|ClearTimerbyFunctionName 0 "Attackk" :!label _label))
          (:NewEnumerator8
            (Default|ChangeAnimStates _anim New%20State 1.0)
            (goto _label))
          (:NewEnumerator9
            (Default|ChangeAnimStates _anim "NewEnumerator9" 1.0))
          (:NewEnumerator10
            (Default|ChangeAnimStates _anim "NewEnumerator10" (Variables|Default|GetAttackSpeed))
            (Utilities|Time|SetTimerbyFunctionName 0 "Attackk" (Variables|Default|GetHeavyAttackStartUpDelay))))))))

(fn ModifyDamage
  (params (Base%20Damage :type Float%20%28double-precision%29))
  (CallFunction|ChangeState "NewEnumerator7")
  (bind _asbp_avatar (Utilities|Casting|CastToBP_Avatar (Game|Player|GetPlayerPawn 0)))
  (if (Variables|/Game/Blueprints/BP_Avatar.BP_Avatar_C|GetHeavyAttackTriggered _asbp_avatar)
    (Variables|Default|SetDamageBonus 2.0)
    (else
      (Variables|Default|SetDamageBonus 1.0)))
  (return (* Base%20Damage (Variables|Default|GetDamageBonus))))

(fn Attackk
  (for _array_element (Collision|GetOverlappingActors (Variables|Default|GetAttackArea) (Variables|Default|GetEnemyClass) :!class /Script/Engine.PrimitiveComponent)
    (if (> (Class|Actor|GetDotProductto _array_element) 0.5)
      (Game|Damage|ApplyDamage _array_element (Variables|Default|GetBaseDamage) 0 0))))