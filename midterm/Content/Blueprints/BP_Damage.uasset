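; BP_Damage is an area hazard actor that deals continuous damage to actors overlapping it.
; A BP_BaseCharacter entering enables Tick, which applies DamagePerSeconds scaled by delta time to every overlapping actor, regardless of class.
; When a character leaves, Tick stays enabled only if any actors still overlap, so damage processing runs on demand.
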(event EventBeginPlay)

(event Collision|EventActorBeginOverlap
  (params (OtherActor :type Actor%20Object%20Reference))
  (Utilities|Casting|CastToBP_BaseCharacter OtherActor)
  (Actor|Tick|SetActorTickEnabled true))

(event EventTick
  (params (DeltaSeconds :type Float%20%28single-precision%29))
  (for _array_element (Collision|GetOverlappingActors 0 :!class /Script/Engine.Actor)
    (Game|Damage|ApplyDamage _array_element (* DeltaSeconds (Variables|Default|GetDamagePerSeconds)) 0 0)))

(event Collision|EventActorEndOverlap
  (params (OtherActor :type Actor%20Object%20Reference))
  (Utilities|Casting|CastToBP_BaseCharacter OtherActor)
  (Actor|Tick|SetActorTickEnabled (> (Utilities|Array|Length (Collision|GetOverlappingActors 0 :!class /Script/Engine.Actor)) 0)))

(fn ConstructionScript)