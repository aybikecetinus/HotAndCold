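; BP_Pond is a hazard actor that teleports to a random spot at a fixed height every five seconds through a self-renewing timer.
; BP_Avatar overlaps with its sphere toggle Tick, which attempts to spawn a BP_Bullet every frame.
; Each shot solves an arc from a random offset around the pond to the avatar, passing the launch velocity as both bullet velocity and spawn location.
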(event OnComponentBeginOverlap(Sphere)
  (params (OverlappedComponent :type Primitive%20Component%20Object%20Reference) (OtherActor :type Actor%20Object%20Reference) (OtherComp :type Primitive%20Component%20Object%20Reference) (OtherBodyIndex :type Integer) (bFromSweep :type Boolean) (SweepResult :type Hit%20Result%20Structure%20%28by%20ref%29))
  (bind _asbp_avatar (Utilities|Casting|CastToBP_Avatar OtherActor))
  (Variables|Default|SetAs%20BP%20Avatar _asbp_avatar)
  (Actor|Tick|SetActorTickEnabled true))

(event OnComponentEndOverlap(Sphere)
  (params (OverlappedComponent :type Primitive%20Component%20Object%20Reference) (OtherActor :type Actor%20Object%20Reference) (OtherComp :type Primitive%20Component%20Object%20Reference) (OtherBodyIndex :type Integer))
  (bind _asbp_avatar (Utilities|Casting|CastToBP_Avatar OtherActor))
  (Variables|Default|SetAs%20BP%20Avatar _asbp_avatar)
  (Actor|Tick|SetActorTickEnabled false))

(event EventBeginPlay
  (CallFunction|ResetPond))

(event Collision|EventActorBeginOverlap
  (params (OtherActor :type Actor%20Object%20Reference)))

(event EventTick
  (params (DeltaSeconds :type Float%20%28single-precision%29))
  (bind _returnvalue (Math|Random|RandomUnitVector))
  (bind _sphere (Variables|Default|GetSphere))
  (bind _sphereradius (Variables|/Script/Engine.SphereComponent|GetSphereRadius _sphere))
  (bind _returnvalue_2 (* _returnvalue _sphereradius))
  (bind _returnvalue_3 (Math|Vector|ClampVectorSize _returnvalue_2 500.03 _sphereradius))
  (Variables|Default|SetDelta%20Seconds DeltaSeconds)
  (bind _as_bp_avatar (Variables|Default|GetAs%20BP%20Avatar)
    (:then
      (bind _output_get (Variables|Default|SetSpawnLoc (+ (Transformation|GetActorLocation) (Math|Vector|MakeVector (.x _returnvalue_3) (.y _returnvalue_3) 0.0))))
      (bind (_outlaunchvelocity _returnvalue_4) (Game|SuggestProjectileVelocityCustomArc _output_get (Transformation|GetActorLocation _as_bp_avatar) 0.0 0.5))
      (if _returnvalue_4
        (Game|SpawnActorfromClass "/Game/Blueprints/BP_Bullet.BP_Bullet_C" (Math|Transform|MakeTransform _outlaunchvelocity "0, 0, 0" "0.500000,0.250000,0.250000") "Undefined" 0 _outlaunchvelocity 0)))
    (:else)))

(fn ConstructionScript)

(fn ResetPond
  (Transformation|Teleport (Math|Vector|MakeVector (Math|Random|RandomFloatinRange -8e+02 8.8e+02) (Math|Random|RandomFloatinRange -8.8e+02 1.03e+03) -1.4e+02) "0, 0, 0")
  (Utilities|Time|SetTimerbyFunctionName 0 "ResetPond" 5.0))