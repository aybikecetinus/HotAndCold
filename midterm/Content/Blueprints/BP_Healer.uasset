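; BP_Healer is a roaming healing zone that restores health to overlapping BP_BaseCharacter actors.
; Each Tick adds the character's own HealingRate scaled by delta time, capped at MaxHealth.
; Character begin overlap enables Tick, and end overlap keeps it on only while overlapping actors remain.
; From BeginPlay, ResetHealer teleports the actor to a random spot at fixed height and re-arms its own timer to move every few seconds.
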(event EventBeginPlay
  (CallFunction|ResetHealer))

(event Collision|EventActorBeginOverlap
  (params (OtherActor :type Actor%20Object%20Reference))
  (Utilities|Casting|CastToBP_BaseCharacter OtherActor)
  (Actor|Tick|SetActorTickEnabled true))

(event EventTick
  (params (DeltaSeconds :type Float%20%28single-precision%29))
  (for _array_element (Collision|GetOverlappingActors 0 :!class /Script/Engine.Actor)
    (bind _asbp_base_character (Utilities|Casting|CastToBP_BaseCharacter _array_element))
    (bind _output_get (Variables|Default|SetAs%20BP%20Base%20Character _asbp_base_character))
    (Variables|/Game/Blueprints/BP_BaseCharacter.BP_BaseCharacter_C|SetHealth _output_get (Math|Float|Min(Float) (+ (Variables|/Game/Blueprints/BP_BaseCharacter.BP_BaseCharacter_C|GetHealth (Variables|Default|GetAs%20BP%20Base%20Character)) (* (Variables|/Game/Blueprints/BP_BaseCharacter.BP_BaseCharacter_C|GetHealingRate (Variables|Default|GetAs%20BP%20Base%20Character)) DeltaSeconds)) (Variables|/Game/Blueprints/BP_BaseCharacter.BP_BaseCharacter_C|GetMaxHealth (Variables|Default|GetAs%20BP%20Base%20Character))))))

(event Collision|EventActorEndOverlap
  (params (OtherActor :type Actor%20Object%20Reference))
  (Utilities|Casting|CastToBP_BaseCharacter OtherActor)
  (Actor|Tick|SetActorTickEnabled (> (Utilities|Array|Length (Collision|GetOverlappingActors 0 :!class /Script/Engine.Actor)) 0)))

(fn ConstructionScript)

(fn ResetHealer
  (Transformation|Teleport (Math|Vector|MakeVector (Math|Random|RandomFloatinRange -8e+02 8e+02) (Math|Random|RandomFloatinRange -1.2e+03 1.07e+03) 1.1e+02) "0, 0, 0")
  (Utilities|Time|SetTimerbyFunctionName 0 "ResetHealer" 5.0))