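; BP_Enemy is an AI enemy character that chases the player and attacks when in range.
; On BeginPlay it assigns itself as owner of its enemy HUD widget and picks a random attack cooldown.
; A looping AIMoveTo targets the player pawn within AttackRadius, changes state on arrival, then waits out the cooldown, retrying shortly after failed requests.
; The loop ends with a state change when either the player or the enemy is dead.
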(event EventBeginPlay
  (|CallParentFunction)
  (Utilities|FlowControl|Sequence
    (:then_0
      (bind _asw_hud_enemy (Utilities|Casting|CastToW_HUD_Enemy (UserInterface|GetUserWidgetObject (Variables|Default|GetWidget))))
      (Variables|/Game/Blueprints/W_HUD_Enemy.W_HUD_Enemy_C|SetOwnerCharacter _asw_hud_enemy self))
    (:then_1
      (Variables|Default|SetAttackCoolDown (Math|Random|RandomFloatinRange 1.0 2.0))
      (bind _asbp_base_character (Utilities|Casting|CastToBP_BaseCharacter (Game|GetPlayerCharacter 0) :!label _label))
      (if (Variables|/Game/Blueprints/BP_BaseCharacter.BP_BaseCharacter_C|GetDead _asbp_base_character)
        (CallFunction|ChangeState "NewEnumerator9")
        (elif (Variables|Default|GetDead)
          (CallFunction|ChangeState "NewEnumerator8")
          (else
            (AI|AIMoveTo (AI|GetAIController self) "0, 0, 0" (Game|Player|GetPlayerPawn 0) (Variables|Default|GetAttackRadius) "Default" "Default" true true
              (:OnRequestFailed
                (Utilities|FlowControl|Delay 0.2)
                (goto _label))
              (:OnMoveFinished
                (CallFunction|ChangeState "NewEnumerator4")
                (Utilities|FlowControl|Delay (Variables|Default|GetAttackCoolDown))
                (goto _label)))))))))

(event Collision|EventActorBeginOverlap
  (params (OtherActor :type Actor%20Object%20Reference))
  (|CallParentFunction OtherActor) ; This node is disabled and will not be called.\nDrag off pins to build functionality.
)

(event EventTick
  (params (DeltaSeconds :type Float%20%28single-precision%29))
  (|CallParentFunction DeltaSeconds) ; This node is disabled and will not be called.\nDrag off pins to build functionality.
)

(fn ConstructionScript
  (|CallParentFunction))